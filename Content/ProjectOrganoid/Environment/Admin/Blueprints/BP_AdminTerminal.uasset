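; BP_AdminTerminal is an interactable admin-area terminal with power state, optional one-shot use and a selectable terminal type.
; Its Interact override calls Activate when the parent interaction succeeds, unless a one-shot terminal is already used.
; Activate turns the status light red if unpowered; otherwise it turns cyan, records use and fires the event matching TerminalType.
; The six type events, from Reception to Transit, are placeholders that only print debug strings.
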(event Custom|Activate
  (if (not (and (Variables|Admin|Terminal|GetbOneShot) (Variables|Admin|Terminal|GetbHasActivated)))
    (if (Variables|Admin|Terminal|GetbIsPowered)
      (CallFunction|ActivateScreen)
      (else
        (CallFunction|PlayErrorFX)))))

(event Custom|PlayErrorFX
  (Rendering|Components|Light|SetLightColor (Variables|Default|GetStatusLight) "(R=1.000000,G=0.120000,B=0.080000,A=1.000000)" true)
  (Development|PrintString "AdminTerminal Error: unpowered" true true "(R=0.000000,G=0.660000,B=1.000000,A=1.000000)" 3.0))

(event Custom|ActivateScreen
  (Rendering|Components|Light|SetLightColor (Variables|Default|GetStatusLight) "(R=0.200000,G=0.850000,B=1.000000,A=1.000000)" true)
  (Development|PrintString "AdminTerminal Screen" true true "(R=0.000000,G=0.660000,B=1.000000,A=1.000000)" 3.0)
  (Variables|Admin|Terminal|SetbHasActivated true)
  (if (Variables|Admin|Terminal|GetbOneShot)
    (Variables|Default|SetbIsInteractable false))
  (switch Utilities|FlowControl|Switch|SwitchonE_AdminTerminalType (Variables|Admin|Terminal|GetTerminalType)
    (:NewEnumerator0
      (CallFunction|OnReceptionActivated))
    (:NewEnumerator1
      (CallFunction|OnSecurityActivated))
    (:NewEnumerator2
      (CallFunction|OnRecordsActivated))
    (:NewEnumerator3
      (CallFunction|OnExecutiveActivated))
    (:NewEnumerator4
      (CallFunction|OnOperationsActivated))
    (:NewEnumerator5
      (CallFunction|OnTransitActivated))))

(event Custom|OnReceptionActivated
  (Development|PrintString "AdminTerminal OnReceptionActivated" true true "(R=0.000000,G=0.660000,B=1.000000,A=1.000000)" 3.0))

(event Custom|OnSecurityActivated
  (Development|PrintString "AdminTerminal OnSecurityActivated" true true "(R=0.000000,G=0.660000,B=1.000000,A=1.000000)" 3.0))

(event Custom|OnRecordsActivated
  (Development|PrintString "AdminTerminal OnRecordsActivated" true true "(R=0.000000,G=0.660000,B=1.000000,A=1.000000)" 3.0))

(event Custom|OnExecutiveActivated
  (Development|PrintString "AdminTerminal OnExecutiveActivated" true true "(R=0.000000,G=0.660000,B=1.000000,A=1.000000)" 3.0))

(event Custom|OnOperationsActivated
  (Development|PrintString "AdminTerminal OnOperationsActivated" true true "(R=0.000000,G=0.660000,B=1.000000,A=1.000000)" 3.0))

(event Custom|OnTransitActivated
  (Development|PrintString "AdminTerminal OnTransitActivated" true true "(R=0.000000,G=0.660000,B=1.000000,A=1.000000)" 3.0))

(event EventBeginPlay
  (Variables|Admin|Terminal|SetbIsPowered (Variables|Admin|Terminal|GetbInitiallyPowered)))

(event Collision|EventActorBeginOverlap
  (params (OtherActor :type Actor%20Object%20Reference)))

(event EventTick
  (params (DeltaSeconds :type Float%20%28single-precision%29)))

(fn ConstructionScript)

(fn Interact
  (params (Interactor :type Project%20Organoid%20Character%20Object%20Reference))
  (if (not (and (Variables|Admin|Terminal|GetbOneShot) (Variables|Admin|Terminal|GetbHasActivated)))
    (bind _returnvalue (|CallParentFunction Interactor))
    (if _returnvalue
      (CallFunction|Activate)
      (return _returnvalue))))