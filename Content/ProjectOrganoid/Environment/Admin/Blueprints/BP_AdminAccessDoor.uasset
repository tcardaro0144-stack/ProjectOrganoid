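; Two-panel sliding access door for the Admin environment that opens when a ProjectOrganoidCharacter overlaps it.
; If Automatic and not yet open, an unlocked door plays a Timeline that lerps both panels apart along relative Y by OpenDistance, then sets IsOpen.
; A locked door turns its status light, cyan at BeginPlay, red instead.
; No closing or unlocking logic exists here, and actor tick is disabled.
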(event EventBeginPlay
  (Variables|Admin|Door|SetClosedLeft (Variables|/Script/Engine.SceneComponent|GetRelativeLocation (Variables|Default|GetDoor_Left)))
  (Variables|Admin|Door|SetClosedRight (Variables|/Script/Engine.SceneComponent|GetRelativeLocation (Variables|Default|GetDoor_Right)))
  (Actor|Tick|SetActorTickEnabled false)
  (Rendering|Components|Light|SetLightColor (Variables|Default|GetStatusLight) "(R=0.200000,G=0.850000,B=1.000000,A=1.000000)" true))

(event Collision|EventActorBeginOverlap
  (params (OtherActor :type Actor%20Object%20Reference))
  (bind _closedleft (Variables|Admin|Door|GetClosedLeft))
  (bind _closedright (Variables|Admin|Door|GetClosedRight))
  (bind _opendistance (Variables|Admin|Door|GetOpenDistance))
  (Utilities|Casting|CastToProjectOrganoidCharacter OtherActor)
  (if (Variables|Admin|Door|GetbAutomatic)
    (if (not (Variables|Admin|Door|GetbIsOpen))
      (if (Variables|Admin|Door|GetbLocked)
        (Rendering|Components|Light|SetLightColor (Variables|Default|GetStatusLight) "(R=1.000000,G=0.120000,B=0.080000,A=1.000000)" true)
        (else
          (bind _alpha (Timeline|Timeline PlayFromStart)
            (:Update
              (Transformation|SetRelativeLocation (Variables|Default|GetDoor_Left) (Math|Vector|Lerp(Vector) _closedleft (+ _closedleft (Math|Vector|MakeVector 0.0 (* _opendistance -1.0) 0.0)) _alpha) false false)
              (Transformation|SetRelativeLocation (Variables|Default|GetDoor_Right) (Math|Vector|Lerp(Vector) _closedright (+ _closedright (Math|Vector|MakeVector 0.0 _opendistance 0.0)) _alpha) false false))
            (:Finished
              (Variables|Admin|Door|SetbIsOpen true))))))))

(fn ConstructionScript)