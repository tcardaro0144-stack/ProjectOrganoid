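; BP_AdminLightController manages zone-based lighting for the Admin environment, tracking the current lighting zone.
; The construction script applies that zone's lighting using the authored intensity and an inactive multiplier.
; SetLightingZone switches zones only for names that pass the approved Admin zone check, then reapplies the lighting.
; BeginPlay, overlap and Tick are unused, so changes after construction come only through SetLightingZone calls.
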(event EventBeginPlay)

(event Collision|EventActorBeginOverlap
  (params (OtherActor :type Actor%20Object%20Reference)))

(event EventTick
  (params (DeltaSeconds :type Float%20%28single-precision%29)))

(fn ConstructionScript
  (Class|ProjectOrganoidAdminLightingLibrary|ApplyAdminZoneLighting (Variables|Admin|Lighting|GetCurrentLightingZone) (Variables|Admin|Lighting|GetAuthoredIntensity) (Variables|Admin|Lighting|GetInactiveMultiplier)))

(fn SetLightingZone
  (params (ZoneName :type Name :default "None"))
  (if (Class|ProjectOrganoidAdminLightingLibrary|IsApprovedAdminLightingZone ZoneName)
    (Variables|Admin|Lighting|SetCurrentLightingZone ZoneName)
    (Class|ProjectOrganoidAdminLightingLibrary|ApplyAdminZoneLighting ZoneName (Variables|Admin|Lighting|GetAuthoredIntensity) (Variables|Admin|Lighting|GetInactiveMultiplier))
    (return)
    (else
      (return))))