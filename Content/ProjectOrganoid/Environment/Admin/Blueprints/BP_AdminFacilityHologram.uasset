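; Admin facility hologram that shows which facility sections (Admin, NeuroGenetics, Cryo, Compute, Reactor) are online.
; ApplyHologramState reads one boolean per section, toggles its Online or Unknown indicator, and sets its light to bright teal or dim slate.
; It runs only from the Construction Script; the event graph is empty, so nothing in this Blueprint refreshes the display during play.
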(event EventBeginPlay)

(event Collision|EventActorBeginOverlap
  (params (OtherActor :type Actor%20Object%20Reference)))

(event EventTick
  (params (DeltaSeconds :type Float%20%28single-precision%29)))

(fn ConstructionScript
  (CallFunction|ApplyHologramState))

(fn ApplyHologramState
  (bind _indicator_admin_online (Variables|Default|GetIndicator_Admin_Online))
  (bind _light_neurogenetics (Variables|Default|GetLight_NeuroGenetics))
  (bind _indicator_neurogenetics_online (Variables|Default|GetIndicator_NeuroGenetics_Online))
  (bind _indicator_neurogenetics_unknown (Variables|Default|GetIndicator_NeuroGenetics_Unknown))
  (bind _light_neurogenetics_2 (Variables|Default|GetLight_NeuroGenetics))
  (bind _indicator_cryo_online (Variables|Default|GetIndicator_Cryo_Online))
  (bind _indicator_cryo_unknown (Variables|Default|GetIndicator_Cryo_Unknown))
  (bind _light_cryo (Variables|Default|GetLight_Cryo))
  (bind _indicator_cryo_online_2 (Variables|Default|GetIndicator_Cryo_Online))
  (bind _indicator_cryo_unknown_2 (Variables|Default|GetIndicator_Cryo_Unknown))
  (bind _indicator_admin_unknown (Variables|Default|GetIndicator_Admin_Unknown))
  (bind _light_cryo_2 (Variables|Default|GetLight_Cryo))
  (bind _indicator_compute_online (Variables|Default|GetIndicator_Compute_Online))
  (bind _indicator_compute_unknown (Variables|Default|GetIndicator_Compute_Unknown))
  (bind _light_compute (Variables|Default|GetLight_Compute))
  (bind _indicator_compute_online_2 (Variables|Default|GetIndicator_Compute_Online))
  (bind _indicator_compute_unknown_2 (Variables|Default|GetIndicator_Compute_Unknown))
  (bind _light_compute_2 (Variables|Default|GetLight_Compute))
  (bind _indicator_reactor_online (Variables|Default|GetIndicator_Reactor_Online))
  (bind _light_admin (Variables|Default|GetLight_Admin))
  (bind _indicator_reactor_unknown (Variables|Default|GetIndicator_Reactor_Unknown))
  (bind _light_reactor (Variables|Default|GetLight_Reactor))
  (bind _indicator_reactor_online_2 (Variables|Default|GetIndicator_Reactor_Online))
  (bind _indicator_reactor_unknown_2 (Variables|Default|GetIndicator_Reactor_Unknown))
  (bind _light_reactor_2 (Variables|Default|GetLight_Reactor))
  (bind _indicator_admin_online_2 (Variables|Default|GetIndicator_Admin_Online))
  (bind _indicator_admin_unknown_2 (Variables|Default|GetIndicator_Admin_Unknown))
  (bind _light_admin_2 (Variables|Default|GetLight_Admin))
  (bind _indicator_neurogenetics_online_2 (Variables|Default|GetIndicator_NeuroGenetics_Online))
  (bind _indicator_neurogenetics_unknown_2 (Variables|Default|GetIndicator_NeuroGenetics_Unknown))
  (Utilities|FlowControl|Sequence
    (:then_0
      (if (Variables|Admin|Hologram|GetbAdminOnline)
        (Rendering|SetVisibility _indicator_admin_online true false)
        (Development|SetHiddeninGame _indicator_admin_online false false)
        (Rendering|SetVisibility _indicator_admin_unknown false false)
        (Development|SetHiddeninGame _indicator_admin_unknown false false)
        (Rendering|Components|Light|SetIntensity _light_admin 8e+03)
        (Rendering|Components|Light|SetLightColor _light_admin "(R=0.150000,G=1.000000,B=0.750000,A=1.000000)" true)
        (else
          (Rendering|SetVisibility _indicator_admin_online_2 false false)
          (Development|SetHiddeninGame _indicator_admin_online_2 false false)
          (Rendering|SetVisibility _indicator_admin_unknown_2 true false)
          (Development|SetHiddeninGame _indicator_admin_unknown_2 false false)
          (Rendering|Components|Light|SetIntensity _light_admin_2 3.5e+02)
          (Rendering|Components|Light|SetLightColor _light_admin_2 "(R=0.120000,G=0.140000,B=0.180000,A=1.000000)" true))))
    (:then_1
      (if (Variables|Admin|Hologram|GetbNeuroGeneticsOnline)
        (Rendering|SetVisibility _indicator_neurogenetics_online_2 true false)
        (Development|SetHiddeninGame _indicator_neurogenetics_online_2 false false)
        (Rendering|SetVisibility _indicator_neurogenetics_unknown_2 false false)
        (Development|SetHiddeninGame _indicator_neurogenetics_unknown_2 false false)
        (Rendering|Components|Light|SetIntensity _light_neurogenetics 8e+03)
        (Rendering|Components|Light|SetLightColor _light_neurogenetics "(R=0.150000,G=1.000000,B=0.750000,A=1.000000)" true)
        (else
          (Rendering|SetVisibility _indicator_neurogenetics_online false false)
          (Development|SetHiddeninGame _indicator_neurogenetics_online false false)
          (Rendering|SetVisibility _indicator_neurogenetics_unknown true false)
          (Development|SetHiddeninGame _indicator_neurogenetics_unknown false false)
          (Rendering|Components|Light|SetIntensity _light_neurogenetics_2 3.5e+02)
          (Rendering|Components|Light|SetLightColor _light_neurogenetics_2 "(R=0.120000,G=0.140000,B=0.180000,A=1.000000)" true))))
    (:then_2
      (if (Variables|Admin|Hologram|GetbCryoOnline)
        (Rendering|SetVisibility _indicator_cryo_online true false)
        (Development|SetHiddeninGame _indicator_cryo_online false false)
        (Rendering|SetVisibility _indicator_cryo_unknown false false)
        (Development|SetHiddeninGame _indicator_cryo_unknown false false)
        (Rendering|Components|Light|SetIntensity _light_cryo 8e+03)
        (Rendering|Components|Light|SetLightColor _light_cryo "(R=0.150000,G=1.000000,B=0.750000,A=1.000000)" true)
        (else
          (Rendering|SetVisibility _indicator_cryo_online_2 false false)
          (Development|SetHiddeninGame _indicator_cryo_online_2 false false)
          (Rendering|SetVisibility _indicator_cryo_unknown_2 true false)
          (Development|SetHiddeninGame _indicator_cryo_unknown_2 false false)
          (Rendering|Components|Light|SetIntensity _light_cryo_2 3.5e+02)
          (Rendering|Components|Light|SetLightColor _light_cryo_2 "(R=0.120000,G=0.140000,B=0.180000,A=1.000000)" true))))
    (:then_3
      (if (Variables|Admin|Hologram|GetbComputeOnline)
        (Rendering|SetVisibility _indicator_compute_online true false)
        (Development|SetHiddeninGame _indicator_compute_online false false)
        (Rendering|SetVisibility _indicator_compute_unknown false false)
        (Development|SetHiddeninGame _indicator_compute_unknown false false)
        (Rendering|Components|Light|SetIntensity _light_compute 8e+03)
        (Rendering|Components|Light|SetLightColor _light_compute "(R=0.150000,G=1.000000,B=0.750000,A=1.000000)" true)
        (else
          (Rendering|SetVisibility _indicator_compute_online_2 false false)
          (Development|SetHiddeninGame _indicator_compute_online_2 false false)
          (Rendering|SetVisibility _indicator_compute_unknown_2 true false)
          (Development|SetHiddeninGame _indicator_compute_unknown_2 false false)
          (Rendering|Components|Light|SetIntensity _light_compute_2 3.5e+02)
          (Rendering|Components|Light|SetLightColor _light_compute_2 "(R=0.120000,G=0.140000,B=0.180000,A=1.000000)" true))))
    (:then_4
      (if (Variables|Admin|Hologram|GetbReactorOnline)
        (Rendering|SetVisibility _indicator_reactor_online true false)
        (Development|SetHiddeninGame _indicator_reactor_online false false)
        (Rendering|SetVisibility _indicator_reactor_unknown false false)
        (Development|SetHiddeninGame _indicator_reactor_unknown false false)
        (Rendering|Components|Light|SetIntensity _light_reactor 8e+03)
        (Rendering|Components|Light|SetLightColor _light_reactor "(R=0.150000,G=1.000000,B=0.750000,A=1.000000)" true)
        (else
          (Rendering|SetVisibility _indicator_reactor_online_2 false false)
          (Development|SetHiddeninGame _indicator_reactor_online_2 false false)
          (Rendering|SetVisibility _indicator_reactor_unknown_2 true false)
          (Development|SetHiddeninGame _indicator_reactor_unknown_2 false false)
          (Rendering|Components|Light|SetIntensity _light_reactor_2 3.5e+02)
          (Rendering|Components|Light|SetLightColor _light_reactor_2 "(R=0.120000,G=0.140000,B=0.180000,A=1.000000)" true))))))